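; Player character for a top-down shooter that faces the cursor, moves, and fires either projectiles or a mana-fed beam.
; Tick drives most logic: combo points set a five-tier level controlling shot pattern, fire delay, beam length and combo decay.
; A line trace scales the beam to its hit, and a dynamic material displays mana.
; MobTenn contact costs life, score and combo; timed events boost speed or waive mana cost.
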(event `SpeedUp`
  (bind _charactermovement (`self.CharacterMovement`))
  (set `CharacterMovementComponent.MaxWalkSpeed` 3000.0 _charactermovement)
  (set `self.IsSpeedUp?` true)
  (`KismetSystemLibrary.Delay` 10.0)
  (set `self.IsSpeedUp?` false)
  (set `CharacterMovementComponent.MaxWalkSpeed` 850.0 _charactermovement))

(event `Double Dammages`)

(event `ManaIllimited`
  (set `self.ManaCost` 0.0)
  (set `self.ManaIsIllimited?` true)
  (`KismetSystemLibrary.Delay` 10.0)
  (set `self.ManaIsIllimited?` false)
  (set `self.ManaCost` 0.5))

(event `self.ReceiveTick`
  (params (DeltaSeconds :type "Float (single-precision)"))
  (bind _returnvalue (`self.K2_GetActorLocation`))
  (bind _returnvalue_2 (`GameplayStatics.GetPlayerCharacter` 0))
  (bind _returnvalue_3 (`GameplayStatics.GetPlayerController` 0))
  (bind _poisition_start_spells (`self.Poisition start Spells`))
  (bind _poisition_start_spells1 (`self.Poisition start Spells1`))
  (bind _poisition_start_spells2 (`self.Poisition start Spells2`))
  (bind _cylinderbeam (`self.CylinderBeam`))
  (bind _manabar (`self.ManaBar`))
  (bind _cylinderbeam_2 (`self.CylinderBeam`))
  (bind _returnvalue_4 (`SceneComponent.K2_GetComponentToWorld` _poisition_start_spells))
  (bind _returnvalue_x (`KismetMathLibrary.BreakVector` (`SceneComponent.K2_GetComponentScale` _cylinderbeam_2)))
  (bind _returnvalue_5 (`SceneComponent.K2_GetComponentToWorld` _poisition_start_spells1))
  (bind _returnvalue_6 (`SceneComponent.K2_GetComponentToWorld` _poisition_start_spells2))
  ;[1 1 1] LevelUp
  (`|ExecutionSequence`
    (:`then_0`
      ;[1 1 1] Beam
      (if (`self.PlayerUseBeam?`)
        (if (`self.PlayerIsShooting?`)
          _
          (elif (>= (`self.Mana`) 1.0)
            (bind _aschat_anim_bp (cast `/Game/Blueprints/Character/Animation/NewAnim/CHAT_ANIM_BP` (`SkeletalMeshComponent.GetAnimInstance` (`self.Mesh`))))
            (`/Game/Blueprints/Character/Animation/NewAnim/CHAT_ANIM_BP.Laser` _aschat_anim_bp)
            (`PrimitiveComponent.SetCollisionEnabled` _cylinderbeam "QueryOnly")
            (`SceneComponent.SetVisibility` (`self.FX_SM_Lazer_Plane`) true false)
            (`SceneComponent.SetVisibility` (`self.LaserBase`) true false)
            (`SceneComponent.SetVisibility` (`self.LaserEnd`) true false)
            (set `self.Mana` (`KismetMathLibrary.FClamp` (- (`self.Mana`) (`self.ManaCost`)) 0.0 100.0))
            (set `self.RaycastActivate` true)
            (else
              (`PrimitiveComponent.SetCollisionEnabled` _cylinderbeam "NoCollision" :!label _label)
              (`SceneComponent.SetVisibility` (`self.FX_SM_Lazer_Plane`) false false)
              (`SceneComponent.SetVisibility` (`self.LaserBase`) false false)
              (`SceneComponent.SetVisibility` (`self.LaserEnd`) false false)
              (set `self.RaycastActivate` false))))
        (else
          (goto _label))))
    (:`then_1`
      ;[1 1 1] Look At Cursor
      (set `PlayerController.bShowMouseCursor` true _returnvalue_3)
      (`self.K2_SetActorRotation` _returnvalue_2 (`KismetMathLibrary.MakeRotator` (.roll (`KismetMathLibrary.FindLookAtRotation` (`self.K2_GetActorLocation` _returnvalue_2) (`.Location` (`GameplayStatics.BreakHitResult` (`PlayerController.GetHitResultUnderCursorByChannel` _returnvalue_3 "TraceTypeQuery1" true))))) 0.0 (.yaw (`KismetMathLibrary.FindLookAtRotation` (`self.K2_GetActorLocation` _returnvalue_2) (`.Location` (`GameplayStatics.BreakHitResult` (`PlayerController.GetHitResultUnderCursorByChannel` _returnvalue_3 "TraceTypeQuery1" true)))))) false))
    (:`then_2`
      ;[1 1 1] Shoot
      (if (`self.PlayerUseBeam?`)
        _
        (elif (`self.PlayerIsShooting?`)
          (if (`self.ShootTime`)
            (bind _aschat_anim_bp_2 (cast `/Game/Blueprints/Character/Animation/NewAnim/CHAT_ANIM_BP` (`SkeletalMeshComponent.GetAnimInstance` (`self.Mesh`))))
            (`/Game/Blueprints/Character/Animation/NewAnim/CHAT_ANIM_BP.SpellShoot` _aschat_anim_bp_2)
            (`GameplayStatics.PlaySound2D` "/Game/Sound/shoot__1_.shoot__1_" 1.0 (`KismetMathLibrary.FClamp` (`KismetMathLibrary.RandomFloat`) -2.0 2.0) 0.0 null null)
            (switch `int` (`self.CurrentLevel`)
              (:`1`
                ;;[1 1 1] Lvl1
                (`GameplayStatics.SpawnEmitterAtLocation` "/Game/Art/FX/Projectile_Muzzle/FX_Projectile_Muzzle.FX_Projectile_Muzzle" (`SceneComponent.K2_GetComponentLocation` (`self.Poisition start Spells`)))
                (`|SpawnActorFromClass` (`self.MyBulletLevel`) _returnvalue_4 "Undefined" "OverrideRootScale" null null)
                (set `self.ShootTime` false)
                (`KismetSystemLibrary.Delay` (`self.ShootDelay`))
                (set `self.ShootTime` true))
              (:`2`
                ;;[1 1 1] Lvl 2
                (`|ExecutionSequence`
                  (:`then_0`
                    (`GameplayStatics.SpawnEmitterAtLocation` "/Game/Art/FX/Projectile_Muzzle/FX_Projectile_Muzzle.FX_Projectile_Muzzle" (`SceneComponent.K2_GetComponentLocation` _poisition_start_spells1))
                    (`|SpawnActorFromClass` (`self.MyBulletLevel`) _returnvalue_5 "Undefined" "OverrideRootScale" null null)
                    (set `self.ShootTime` false)
                    (`KismetSystemLibrary.Delay` (`self.ShootDelay`))
                    (set `self.ShootTime` true))
                  (:`then_1`
                    (`GameplayStatics.SpawnEmitterAtLocation` "/Game/Art/FX/Projectile_Muzzle/FX_Projectile_Muzzle.FX_Projectile_Muzzle" (`SceneComponent.K2_GetComponentLocation` _poisition_start_spells2))
                    (`|SpawnActorFromClass` (`self.MyBulletLevel`) _returnvalue_6 "Undefined" "OverrideRootScale" null null)
                    (set `self.ShootTime` false)
                    (`KismetSystemLibrary.Delay` (`self.ShootDelay`))
                    (set `self.ShootTime` true))))
              (:`3`
                ;;[1 1 1] Lvl 3
                (`|ExecutionSequence`
                  (:`then_0`
                    (`GameplayStatics.SpawnEmitterAtLocation` "/Game/Art/FX/Projectile_Muzzle/FX_Projectile_Muzzle.FX_Projectile_Muzzle" (`SceneComponent.K2_GetComponentLocation` _poisition_start_spells1))
                    (`|SpawnActorFromClass` (`self.MyBulletLevel`) _returnvalue_5 "Undefined" "OverrideRootScale" null null)
                    (set `self.ShootTime` false)
                    (`KismetSystemLibrary.Delay` (`self.ShootDelay`))
                    (set `self.ShootTime` true))
                  (:`then_1`
                    (`GameplayStatics.SpawnEmitterAtLocation` "/Game/Art/FX/Projectile_Muzzle/FX_Projectile_Muzzle.FX_Projectile_Muzzle" (`SceneComponent.K2_GetComponentLocation` _poisition_start_spells2))
                    (`|SpawnActorFromClass` (`self.MyBulletLevel`) _returnvalue_6 "Undefined" "OverrideRootScale" null null)
                    (set `self.ShootTime` false)
                    (`KismetSystemLibrary.Delay` (`self.ShootDelay`))
                    (set `self.ShootTime` true))
                  (:`then_2`
                    (`GameplayStatics.SpawnEmitterAtLocation` "/Game/Art/FX/Projectile_Muzzle/FX_Projectile_Muzzle.FX_Projectile_Muzzle" (`SceneComponent.K2_GetComponentLocation` _poisition_start_spells))
                    (`|SpawnActorFromClass` (`self.MyBulletLevel`) _returnvalue_4 "Undefined" "OverrideRootScale" null null)
                    (set `self.ShootTime` false)
                    (`KismetSystemLibrary.Delay` (`self.ShootDelay`))
                    (set `self.ShootTime` true))))
              (:`4`
                ;;[1 1 1] Lvl 4
                (`|ExecutionSequence`
                  (:`then_0`
                    (`GameplayStatics.SpawnEmitterAtLocation` "/Game/Art/FX/Projectile_Muzzle/FX_Projectile_Muzzle.FX_Projectile_Muzzle" (`SceneComponent.K2_GetComponentLocation` _poisition_start_spells))
                    (`|SpawnActorFromClass` (`self.MyBulletLevel`) _returnvalue_5 "Undefined" "OverrideRootScale" null null)
                    (set `self.ShootTime` false)
                    (`KismetSystemLibrary.Delay` (`self.ShootDelay`))
                    (set `self.ShootTime` true))
                  (:`then_1`
                    (`GameplayStatics.SpawnEmitterAtLocation` "/Game/Art/FX/Projectile_Muzzle/FX_Projectile_Muzzle.FX_Projectile_Muzzle" (`SceneComponent.K2_GetComponentLocation` _poisition_start_spells1))
                    (`|SpawnActorFromClass` (`self.MyBulletLevel`) _returnvalue_6 "Undefined" "OverrideRootScale" null null)
                    (set `self.ShootTime` false)
                    (`KismetSystemLibrary.Delay` (`self.ShootDelay`))
                    (set `self.ShootTime` true))
                  (:`then_2`
                    (`GameplayStatics.SpawnEmitterAtLocation` "/Game/Art/FX/Projectile_Muzzle/FX_Projectile_Muzzle.FX_Projectile_Muzzle" (`SceneComponent.K2_GetComponentLocation` _poisition_start_spells2))
                    (`|SpawnActorFromClass` (`self.MyBulletLevel`) _returnvalue_4 "Undefined" "OverrideRootScale" null null)
                    (set `self.ShootTime` false)
                    (`KismetSystemLibrary.Delay` (`self.ShootDelay`))
                    (set `self.ShootTime` true))))
              (:`5`
                ;;[1 1 1] Lvl 5
                (`GameplayStatics.SpawnEmitterAtLocation` "/Game/Art/FX/Projectile_Muzzle/FX_Projectile_Muzzle.FX_Projectile_Muzzle" (`SceneComponent.K2_GetComponentLocation` _poisition_start_spells))
                (`|SpawnActorFromClass` "/Game/Blueprints/Character/Bullets/BulletReactivation.BulletReactivation_C" _returnvalue_4 "Undefined" "OverrideRootScale" null null)
                (set `self.ShootTime` false)
                (`KismetSystemLibrary.Delay` (`self.ShootDelay`))
                (set `self.ShootTime` true)))))))
    (:`then_3`
      (switch `int` (`self.CurrentLevel`)
        (:`1`
          (set `self.MyBulletLevel` "/Game/Blueprints/Character/Bullets/BulletTest.BulletTest_C")
          (`/Engine/EditorBlueprintResources/StandardMacros.Gate` false
            (:`Exit`
              (set `self.RaycastLenght` 15.0)
              (set `self.ShootDelay` 0.7)
              (if (not (`self.CurrentLevelDelaiCheck`))
                (set `self.ComboPoints` (- (`self.ComboPoints`) 0.2))
                (set `self.CurrentLevelDelaiCheck` true)
                (`KismetSystemLibrary.Delay` 1.0)
                (set `self.CurrentLevelDelaiCheck` false)))))
        (:`2`
          (set `self.MyBulletLevel` "/Game/Blueprints/Character/Bullets/BulletTest.BulletTest_C")
          (`/Engine/EditorBlueprintResources/StandardMacros.Gate` false
            (:`Exit`
              (set `self.RaycastLenght` 20.0)
              (set `self.ShootDelay` 0.6)
              (if (not (`self.CurrentLevelDelaiCheck`))
                (set `self.ComboPoints` (- (`self.ComboPoints`) 0.2))
                (set `self.CurrentLevelDelaiCheck` true)
                (`KismetSystemLibrary.Delay` 1.0)
                (set `self.CurrentLevelDelaiCheck` false)))))
        (:`3`
          (set `self.MyBulletLevel` "/Game/Blueprints/Character/Bullets/BulletTest.BulletTest_C")
          (`/Engine/EditorBlueprintResources/StandardMacros.Gate` false
            (:`Exit`
              (set `self.RaycastLenght` 25.0)
              (set `self.ShootDelay` 0.5)
              (if (not (`self.CurrentLevelDelaiCheck`))
                (set `self.ComboPoints` (- (`self.ComboPoints`) 0.5))
                (set `self.CurrentLevelDelaiCheck` true)
                (`KismetSystemLibrary.Delay` 1.0)
                (set `self.CurrentLevelDelaiCheck` false)))))
        (:`4`
          (set `self.MyBulletLevel` "/Game/Blueprints/Character/Bullets/BulletTest.BulletTest_C")
          (`/Engine/EditorBlueprintResources/StandardMacros.Gate` false
            (:`Exit`
              (set `self.RaycastLenght` 30.0)
              (set `self.ShootDelay` 0.4)
              (if (not (`self.CurrentLevelDelaiCheck`))
                (set `self.ComboPoints` (- (`self.ComboPoints`) 1.0))
                (set `self.CurrentLevelDelaiCheck` true)
                (`KismetSystemLibrary.Delay` 1.0)
                (set `self.CurrentLevelDelaiCheck` false)))))
        (:`5`
          (set `self.MyBulletLevel` "/Game/Blueprints/Character/Bullets/BulletTest.BulletTest_C")
          (`/Engine/EditorBlueprintResources/StandardMacros.Gate` false
            (:`Exit`
              (set `self.RaycastLenght` 40.0)
              (set `self.ShootDelay` 0.6)
              (if (not (`self.CurrentLevelDelaiCheck`))
                (set `self.ComboPoints` (- (`self.ComboPoints`) 2.0))
                (set `self.CurrentLevelDelaiCheck` true)
                (`KismetSystemLibrary.Delay` 1.0)
                (set `self.CurrentLevelDelaiCheck` false)))))))
    (:`then_4`
      ;[1 1 1] Combo Systeme
      (`|ExecutionSequence`
        (:`then_0`
          (set `self.ComboPoints` (`KismetMathLibrary.FClamp` (`self.ComboPoints`) 0.0 60.0)))
        (:`then_1`
          (set `self.CurrentLevel` (`KismetMathLibrary.Clamp` (`KismetMathLibrary.FTrunc` (/ (`self.ComboPoints`) 10.0)) 1 5)))))
    (:`then_5`
      ;[1 1 1] ManaBarMatInstance
      (bind _returnvalue_7 (`PrimitiveComponent.CreateDynamicMaterialInstance` _manabar 0 (`PrimitiveComponent.GetMaterial` _manabar 0) "None"))
      (`MaterialInstanceDynamic.SetScalarParameterValue` _returnvalue_7 "Decimal" (/ (`self.Mana`) 100.0))
      (`MaterialInstanceDynamic.SetVectorParameterValue` _returnvalue_7 "Color" (struct :`R` 0.191156 :`G` 0.345371 :`B` 0.708333 :`A` 0.8)))
    (:`then_6`
      (if (not (`self.PlayerUseBeam?`))
        (set `self.Mana` (`KismetMathLibrary.FClamp` (+ (`self.Mana`) 0.08) 0.0 100.0))))
    (:`then_7`
      ;[1 1 1] World rotation mana bar
      (`SceneComponent.K2_SetWorldRotation` (`self.ManaBar`) (`self.ManaBarRotation`) false false))
    (:`then_9`
      ;[1 1 1] Scale Laser by hit
      (if (`self.RaycastActivate`)
        (`GameplayStatics.PlayWorldCameraShake` "/Game/Blueprints/Character/CameraShakeLasezr.CameraShakeLasezr_C" (`self.K2_GetActorLocation`) 3000.0)
        (bind _outactors (`GameplayStatics.GetAllActorsOfClass` "/Game/Blueprints/NPC/MobTenn.MobTenn_C"))
        (bind _outactors_2 (`GameplayStatics.GetAllActorsOfClass` "/Game/Blueprints/Prefab/XP_Collectible.XP_Collectible_C"))
        (set `self.ArrayOfActoreToIgnore` _outactors)
        (bind _outhit (`KismetSystemLibrary.LineTraceSingle` _returnvalue (+ (* (`self.GetActorForwardVector`) 1000.0) _returnvalue) "TraceTypeQuery1" false _outactors_2))
        (bind (_bblockinghit _binitialoverlap _time _distance _location _impactpoint) (`GameplayStatics.BreakHitResult` _outhit))
        (if _bblockinghit
          (`SceneComponent.SetWorldScale3D` (`self.CylinderBeam`) (`KismetMathLibrary.MakeVector` (`KismetMathLibrary.FClamp` (/ (`KismetMathLibrary.VSize` (- _returnvalue _impactpoint)) 25.0) 0.0 _returnvalue_x) 2.3 2.3))
          (else
            (`SceneComponent.SetWorldScale3D` _cylinderbeam_2 (`KismetMathLibrary.MakeVector` (`self.RaycastLenght`) 2.3 2.3))))))
    (:`then_10`
      ;[1 1 1] Loose
      (if (<= (`self.LifePlayer`) 0)
        (`KismetSystemLibrary.PrintString` "LOOOOOOOOOOOOOOOOOOSSSSSERRRRRRRRRRRRRRRR" true true (struct :`R` 0.682292 :`G` 0.13278 :`B` 0.180354 :`A` 1.0) 25.0)))))

(event `self.ReceiveBeginPlay`
  ;[1 1 1] World rotation mana bar
  (`|ExecutionSequence`
    (:`then_0`
      (set `self.ManaBarRotation` (`SceneComponent.K2_GetComponentRotation` (`self.ManaBar`))))
    (:`then_1`
      (bind _returnvalue (`|CreateWidget` "/Game/Blueprints/HUD/HUD.HUD_C"))
      (`UserWidget.AddToViewport` _returnvalue 0))
    (:`then_2`
      (`GameplayStatics.CreateSound2D` "/Game/Sound/beam.beam" 1.0 1.0 0.0 null))))

(event `InputAxis|MoveRight`
  (params (AxisValue :type "Float (single-precision)"))
  ;[1 1 1] Mouvements
  (`self.AddMovementInput` (`GameplayStatics.GetPlayerCharacter` 0) (0.0 90.0 0.0) AxisValue false))

(event `InputAxis|MoveForward`
  (params (AxisValue :type "Float (single-precision)"))
  ;[1 1 1] Mouvements
  (`self.AddMovementInput` (`GameplayStatics.GetPlayerCharacter` 0) (90.0 0.0 0.0) AxisValue false))

(event `InputAction|Fire`
  (params (Key :type "Key Structure"))
  ;[1 1 1] Input
  (:`Pressed`
    (set `self.PlayerIsShooting?` true))
  (:`Released`
    (set `self.PlayerIsShooting?` false)))

(event `InputAction|Beam`
  (params (Key :type "Key Structure"))
  ;[1 1 1] Input
  (:`Pressed`
    (set `self.PlayerUseBeam?` true)
    (bind _returnvalue (`AddComponent|NODE_AddAudioComponent-2`))
    (`AudioComponent.SetVolumeMultiplier` _returnvalue 1.0))
  (:`Released`
    (set `self.PlayerUseBeam?` false)
    (`AudioComponent.SetVolumeMultiplier` _returnvalue 0.0)))

(event `InputAction|Reactivation`
  (params (Key :type "Key Structure"))
  ;[1 1 1] Input
  (:`Pressed`
    (set `self.ReactivationEnable` true)
    (`KismetSystemLibrary.Delay` 0.05)
    (set `self.ReactivationEnable` false)))

(event `self.CapsuleComponent.OnComponentBeginOverlap`
  (params (OverlappedComponent :type "PrimitiveComponent Object Reference") (OtherActor :type "Actor Object Reference") (OtherComp :type "PrimitiveComponent Object Reference") (OtherBodyIndex :type Integer) (bFromSweep :type Boolean) (SweepResult :type "HitResult Structure (by ref)"))
  ;[1 1 1] TakeDammages
  (bind _asmob_tenn (cast `/Game/Blueprints/NPC/MobTenn` OtherActor)
    (:`then`
      (`/Engine/EditorBlueprintResources/StandardMacros.DoOnce` false :!label _label_2
        (:`Completed`
          (bind _aschat_anim_bp (cast `/Game/Blueprints/Character/Animation/NewAnim/CHAT_ANIM_BP` (`SkeletalMeshComponent.GetAnimInstance` (`self.Mesh`))))
          (`/Game/Blueprints/Character/Animation/NewAnim/CHAT_ANIM_BP.TakeDammage` _aschat_anim_bp)
          (set `/Game/Blueprints/NPC/MobTenn.Life` 0.0 _asmob_tenn)
          (`GameplayStatics.PlayWorldCameraShake` "/Game/Blueprints/Character/TakeDammageCameraShake.TakeDammageCameraShake_C" (`self.K2_GetActorLocation`) 3000.0)
          (bind (_returnvalue_x _returnvalue_y) (`KismetMathLibrary.BreakVector` (* (`KismetMathLibrary.Normal` (- (`self.K2_GetActorLocation`) (`self.K2_GetActorLocation` _asmob_tenn))) 300.0)))
          (`self.LaunchCharacter` (`KismetMathLibrary.MakeVector` _returnvalue_x _returnvalue_y 100.0))
          (`/Game/Blueprints/NPC/MobTenn.CheckLife` _asmob_tenn)
          (set `self.Score` (- (`self.Score`) 50))
          (set `self.ComboPoints` (- (`self.ComboPoints`) 5.0))
          (set `self.LifePlayer` (- (`self.LifePlayer`) 1)))))
    (:`CastFailed`
      (goto _label_2 :!via `Reset`))))

(fn `UserConstructionScript`)