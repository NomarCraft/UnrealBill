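; XP pickup actor that flies toward the player and adds to their ComboPoints when collected.
; Each Tick within range, it faces away from Charactertest and steps backward along its forward vector, a fixed distance per frame not scaled by delta time.
; Overlap between its Capsule and the character's capsule adds the points, spawns a shockwave effect at the character, then destroys the pickup after a short delay.
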(event `self.ReceiveTick`
  (params (DeltaSeconds :type "Float (single-precision)"))
  (if (<= (`self.GetDistanceTo` (`GameplayStatics.GetPlayerCharacter` 0)) 600.0)
    (bind _ascharactertest (cast `/Game/Blueprints/Character/Charactertest` (`GameplayStatics.GetPlayerCharacter` 0)))
    (`self.K2_SetActorRotation` (`KismetMathLibrary.FindLookAtRotation` (`self.K2_GetActorLocation` _ascharactertest) (`self.K2_GetActorLocation`)))
    (`self.K2_AddActorWorldTransform` (`KismetMathLibrary.Conv_VectorToTransform` (* (`self.GetActorForwardVector`) -10.0)))))

(event `self.Capsule.OnComponentBeginOverlap`
  (params (OverlappedComponent :type "PrimitiveComponent Object Reference") (OtherActor :type "Actor Object Reference") (OtherComp :type "PrimitiveComponent Object Reference") (OtherBodyIndex :type Integer) (bFromSweep :type Boolean) (SweepResult :type "HitResult Structure (by ref)"))
  (bind _ascharactertest (cast `/Game/Blueprints/Character/Charactertest` OtherActor))
  (bind _capsulecomponent (`Character.CapsuleComponent` _ascharactertest))
  (if (== OtherComp _capsulecomponent)
    (set `/Game/Blueprints/Character/Charactertest.ComboPoints` (+ (`/Game/Blueprints/Character/Charactertest.ComboPoints` _ascharactertest) 20.0) _ascharactertest)
    (bind (_returnvalue_location _returnvalue_rotation) (`KismetMathLibrary.BreakTransform` (`SceneComponent.K2_GetComponentToWorld` _capsulecomponent)))
    (`GameplayStatics.SpawnEmitterAtLocation` "/Game/Art/FX/Experience/FX_Experience_Shockwave_2.FX_Experience_Shockwave_2" _returnvalue_location _returnvalue_rotation)
    (`KismetSystemLibrary.Delay` 0.05)
    (`self.K2_DestroyActor`)))

(fn `UserConstructionScript`)