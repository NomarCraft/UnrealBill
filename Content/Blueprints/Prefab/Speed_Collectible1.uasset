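; Speed boost collectible that homes in on the player character and grants a speed-up when touched.
; Each tick within 500 units, it faces away from Charactertest and steps backward along its forward vector, drawing it toward the player at a frame-rate-dependent rate.
; Overlap between its capsule and the character's capsule component calls SpeedUp on the character, then destroys the pickup after a brief delay.
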(event `self.ReceiveTick`
  (params (DeltaSeconds :type "Float (single-precision)"))
  (if (<= (`self.GetDistanceTo` (`GameplayStatics.GetPlayerCharacter` 0)) 500.0)
    (bind _ascharactertest (cast `/Game/Blueprints/Character/Charactertest` (`GameplayStatics.GetPlayerCharacter` 0)))
    (`self.K2_SetActorRotation` (`KismetMathLibrary.FindLookAtRotation` (`self.K2_GetActorLocation` _ascharactertest) (`self.K2_GetActorLocation`)))
    (`self.K2_AddActorWorldTransform` (`KismetMathLibrary.Conv_VectorToTransform` (* (`self.GetActorForwardVector`) -5.0)))))

(event `self.Capsule.OnComponentBeginOverlap`
  (params (OverlappedComponent :type "PrimitiveComponent Object Reference") (OtherActor :type "Actor Object Reference") (OtherComp :type "PrimitiveComponent Object Reference") (OtherBodyIndex :type Integer) (bFromSweep :type Boolean) (SweepResult :type "HitResult Structure (by ref)"))
  (bind _ascharactertest (cast `/Game/Blueprints/Character/Charactertest` OtherActor))
  (if (== OtherComp (`Character.CapsuleComponent` _ascharactertest))
    (`|ExecutionSequence`
      (:`then_0`
        (`/Game/Blueprints/Character/Charactertest.SpeedUp` _ascharactertest))
      (:`then_1`
        (`KismetSystemLibrary.Delay` 0.05)
        (`self.K2_DestroyActor`)))))

(fn `UserConstructionScript`)