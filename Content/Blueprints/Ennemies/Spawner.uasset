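; Spawner actor that releases waves of ghost enemies defined in SpawnerData.
; Tick starts the next wave once the previous one has finished spawning and MobWaveCount is back at zero.
; SpawnWave calls itself after each per-entry delay, passing ghost type and position index to SpawnMob.
; SpawnMob spawns MobTenn, Splitter or Intangiblebleble at the indexed SpawnerPositions location and gives each a reference to the spawner.
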(event `self.ReceiveTick`
  (params (DeltaSeconds :type "Float (single-precision)"))
  (bind (_waves _wavecount) (break `/Game/Blueprints/Ennemies/WavesData` (`self.SpawnerData`)))
  (if (`self.WaveCompleted`)
    (if (== (`self.MobWaveCount`) 0)
      (if (<= (`self.WaveCount`) _wavecount)
        (set `self.WaveCompleted` false)
        (`self.SpawnWave` (`|GetArrayItem` _waves (`self.WaveCount`)))))))

(event `self.ReceiveBeginPlay`)

(event `SpawnWave`
  (params (Wave :type "/Game/Blueprints/Ennemies/MobSpawning Structure"))
  (bind _wave (break `/Game/Blueprints/Ennemies/MobSpawning` Wave))
  (bind _returnvalue (`KismetArrayLibrary.Array_Length` _wave))
  (bind (_ghosttype _timeuntilspawn _spawnnumber) (break `/Game/Blueprints/Ennemies/MobSpawningElement` (`|GetArrayItem` _wave (`self.CurrentWaveCount`))))
  (if (== (`self.CurrentWaveCount`) 0)
    (set `self.MobWaveCount` _returnvalue)
    (set `self.CurrentWaveLength` _returnvalue))
  (set `self.CurrentWaveCount` (+ (`self.CurrentWaveCount`) 1))
  (`KismetSystemLibrary.Delay` _timeuntilspawn)
  (`self.SpawnMob` _ghosttype _spawnnumber)
  (if (< (`self.CurrentWaveCount`) (`self.CurrentWaveLength`))
    (`self.SpawnWave` (`|GetArrayItem` (`.Waves_6_BE87F8154B26911751B194894FA0EAB5` (break `/Game/Blueprints/Ennemies/WavesData` (`self.SpawnerData`))) (`self.WaveCount`)))
    (else
      (set `self.CurrentWaveCount` 0)
      (`KismetSystemLibrary.PrintString` "put1")
      (set `self.WaveCount` (+ (`self.WaveCount`) 1))
      (set `self.WaveCompleted` true))))

(fn `SpawnMob`
  (params (MobType :type "/Game/Blueprints/Ennemies/MobTypes Enum" :default "NewEnumerator0") (SpawnPos :type Integer))
  (bind _output_location (`KismetMathLibrary.BreakTransform` (`|GetArrayItem` (`self.SpawnerPositions`) SpawnPos)))
  (if (`|EnumEquality` MobType "NewEnumerator0")
    (bind _returnvalue (`|SpawnActorFromClass` "/Game/Blueprints/NPC/MobTenn.MobTenn_C" (`KismetMathLibrary.MakeTransform` _output_location) "AlwaysSpawn" "OverrideRootScale" null null))
    (set `/Game/Blueprints/NPC/MobTenn.SpawnerRef` self _returnvalue)
    (elif (`|EnumEquality` MobType "NewEnumerator1")
      (`KismetSystemLibrary.PrintString` "Splitter")
      (bind _returnvalue_2 (`|SpawnActorFromClass` "/Game/Blueprints/NPC/Splitter.Splitter_C" (`KismetMathLibrary.MakeTransform` _output_location) "AlwaysSpawn" "OverrideRootScale" null null))
      (set `/Game/Blueprints/NPC/MobTenn.SpawnerRef` self _returnvalue_2)
      (elif (`|EnumEquality` MobType "NewEnumerator2")
        (`KismetSystemLibrary.PrintString` "Intangible")
        (bind _returnvalue_3 (`|SpawnActorFromClass` "/Game/Blueprints/NPC/intangiblebleble.intangiblebleble_C" (`KismetMathLibrary.MakeTransform` _output_location) "AlwaysSpawn" "OverrideRootScale" null null))
        (set `/Game/Blueprints/NPC/MobTenn.SpawnerRef` self _returnvalue_3)))))

(fn `UserConstructionScript`)