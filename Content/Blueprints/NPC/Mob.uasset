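; Enemy mob that chases the player character and is destroyed when its Life runs out.
; Tick turns it toward the player, moves it forward by Speed without sweep, checks Life, and writes an empty EnemyLife to its life bar widget.
; Capsule overlaps with three bullet types or the player's beam cylinder reduce Life, gated by short Delay-reset flags.
; Bullets are destroyed on hit; only BulletTest also offsets the mob's position.
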(event `self.ReceiveTick`
  (params (DeltaSeconds :type "Float (single-precision)"))
  (`|ExecutionSequence`
    (:`then_0`
      (bind _aslife_bar_npc (cast `/Game/Blueprints/NPC/LifeBarNPC` (`WidgetComponent.GetUserWidgetObject` (`self.LifeBar`))))
      (set `/Game/Blueprints/NPC/LifeBarNPC.EnemyLife` null _aslife_bar_npc))
    (:`then_1`
      (bind _ascharactertest (cast `/Game/Blueprints/Character/Charactertest` (`GameplayStatics.GetPlayerCharacter` 0)))
      (`self.K2_SetActorRotation` (`KismetMathLibrary.FindLookAtRotation` (`self.K2_GetActorLocation`) (`self.K2_GetActorLocation` _ascharactertest)))
      (`self.K2_AddActorWorldTransform` (`KismetMathLibrary.Conv_VectorToTransform` (* (`self.GetActorForwardVector`) (`self.Speed`)))))
    (:`then_2`
      (if (<= (`self.Life`) 0.0)
        (`self.K2_DestroyActor`)))))

(event `self.Capsule.OnComponentBeginOverlap`
  (params (OverlappedComponent :type "PrimitiveComponent Object Reference") (OtherActor :type "Actor Object Reference") (OtherComp :type "PrimitiveComponent Object Reference") (OtherBodyIndex :type Integer) (bFromSweep :type Boolean) (SweepResult :type "HitResult Structure (by ref)"))
  (`|ExecutionSequence`
    (:`then_0`
      (if (not (`self.TimerInvisibilite`))
        (bind _asbullet_test (cast `/Game/Blueprints/Character/Bullets/BulletTest` OtherActor))
        (`self.K2_DestroyActor` _asbullet_test)
        (set `self.Life` (- (`self.Life`) 0.1))
        (set `self.TimerInvisibilite` true)
        (`self.K2_AddActorWorldTransform` (`KismetMathLibrary.Conv_VectorToTransform` (- (`KismetMathLibrary.VLerp` (`self.GetActorForwardVector`) (`SceneComponent.K2_GetComponentLocation` (`self.Capsule`)) 0.1) -1.0)))
        (`KismetSystemLibrary.Delay` 0.2)
        (set `self.TimerInvisibilite` false)))
    (:`then_1`
      (bind _ascharactertest (cast `/Game/Blueprints/Character/Charactertest` OtherActor))
      (if (== OtherComp (`/Game/Blueprints/Character/Charactertest.BeamCylinder` _ascharactertest))
        (if (not (`self.BEamDelay`))
          (set `self.Life` (- (`self.Life`) 0.1))
          (set `self.BEamDelay` true)
          (`KismetSystemLibrary.Delay` 0.5)
          (set `self.BEamDelay` false))))
    (:`then_2`
      (if (not (`self.TimerInvisibilite`))
        (bind _asbullet_double (cast `/Game/Blueprints/Character/Bullets/BulletDouble` OtherActor))
        (`self.K2_DestroyActor` _asbullet_double)
        (set `self.Life` (- (`self.Life`) 0.1))
        (set `self.TimerInvisibilite` true)
        (`KismetSystemLibrary.Delay` 0.2)
        (set `self.TimerInvisibilite` false)))
    (:`then_3`
      (if (not (`self.TimerInvisibilite`))
        (bind _asbullet_scale (cast `/Game/Blueprints/Character/Bullets/BulletScale` OtherActor))
        (`self.K2_DestroyActor` _asbullet_scale)
        (set `self.Life` (- (`self.Life`) 0.1))
        (set `self.TimerInvisibilite` true)
        (`KismetSystemLibrary.Delay` 0.2)
        (set `self.TimerInvisibilite` false)))))

(fn `UserConstructionScript`)