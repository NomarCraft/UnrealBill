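; MobMartin is an enemy NPC that moves toward the player and dies when its life drops below zero.
; Tick always calls SimpleMoveToActor; once PawnSensing spots the player, it also turns to face them on the horizontal plane.
; Capsule overlaps with three bullet types or the player's beam reduce Life, throttled by short delay flags, with BulletTest also displacing the mob.
; CheckLife links the mob to its LifeBarNPC widget and handles destruction.
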(event `self.PawnSensing.OnSeePawn`
  (params (Pawn :type "Pawn Object Reference"))
  (cast `/Game/Blueprints/Character/Charactertest` Pawn)
  (set `self.PlayerInSight` true))

(event `self.ReceiveTick`
  (params (DeltaSeconds :type "Float (single-precision)"))
  (bind _returnvalue (`self.K2_GetActorLocation`))
  (`|ExecutionSequence`
    (:`then_0`
      (bind _ascharactertest (cast `/Game/Blueprints/Character/Charactertest` (`GameplayStatics.GetPlayerCharacter` 0)))
      (if (`self.PlayerInSight`)
        (`self.K2_SetActorRotation` (`KismetMathLibrary.FindLookAtRotation` _returnvalue (`KismetMathLibrary.MakeVector` (.x (`self.K2_GetActorLocation` _ascharactertest)) (.y (`self.K2_GetActorLocation` _ascharactertest)) (.z _returnvalue))))
        (`AIBlueprintHelperLibrary.SimpleMoveToActor` (`self.GetController`) _ascharactertest)
        (else
          (`AIBlueprintHelperLibrary.SimpleMoveToActor` (`self.GetController`) _ascharactertest))))
    (:`then_1`
      (`/Engine/EditorBlueprintResources/StandardMacros.DoOnce` false
        (:`Completed`
          (`self.CheckLife`))))))

(event `self.Capsule.OnComponentBeginOverlap`
  (params (OverlappedComponent :type "PrimitiveComponent Object Reference") (OtherActor :type "Actor Object Reference") (OtherComp :type "PrimitiveComponent Object Reference") (OtherBodyIndex :type Integer) (bFromSweep :type Boolean) (SweepResult :type "HitResult Structure (by ref)"))
  (`|ExecutionSequence`
    (:`then_0`
      (if (not (`self.TimerInvisibilite`))
        (bind _asbullet_test (cast `/Game/Blueprints/Character/Bullets/BulletTest` OtherActor))
        (`/Engine/EditorBlueprintResources/StandardMacros.IsValid` _asbullet_test
          (:`Is Valid`
            (`self.K2_DestroyActor` _asbullet_test)
            (set `self.Life` (- (`self.Life`) 0.1))
            (set `self.TimerInvisibilite` true)
            (`self.K2_AddActorWorldTransform` (`KismetMathLibrary.Conv_VectorToTransform` (- (`KismetMathLibrary.VLerp` (`self.GetActorForwardVector`) (`SceneComponent.K2_GetComponentLocation` (`self.Capsule`)) 0.1) -1.0)))
            (`KismetSystemLibrary.Delay` 0.2)
            (set `self.TimerInvisibilite` false)))))
    (:`then_1`
      (bind _ascharactertest (cast `/Game/Blueprints/Character/Charactertest` OtherActor))
      (if (== OtherComp (`/Game/Blueprints/Character/Charactertest.BeamCylinder` _ascharactertest))
        (if (not (`self.BEamDelay`))
          (set `self.Life` (- (`self.Life`) 0.1))
          (set `self.BEamDelay` true)
          (`KismetSystemLibrary.Delay` 0.5)
          (set `self.BEamDelay` false))))
    (:`then_2`
      (if (not (`self.TimerInvisibilite`))
        (bind _asbullet_double (cast `/Game/Blueprints/Character/Bullets/BulletDouble` OtherActor))
        (`self.K2_DestroyActor` _asbullet_double)
        (set `self.Life` (- (`self.Life`) 0.1))
        (set `self.TimerInvisibilite` true)
        (`KismetSystemLibrary.Delay` 0.2)
        (set `self.TimerInvisibilite` false)))
    (:`then_3`
      (if (not (`self.TimerInvisibilite`))
        (bind _asbullet_scale (cast `/Game/Blueprints/Character/Bullets/BulletScale` OtherActor))
        (`self.K2_DestroyActor` _asbullet_scale)
        (set `self.Life` (- (`self.Life`) 0.1))
        (set `self.TimerInvisibilite` true)
        (`KismetSystemLibrary.Delay` 0.2)
        (set `self.TimerInvisibilite` false)))
    (:`then_4`
      (`self.CheckLife`))))

(fn `CheckLife`
  (`|ExecutionSequence`
    (:`then_0`
      (bind _aslife_bar_npc (cast `/Game/Blueprints/NPC/LifeBarNPC` (`WidgetComponent.GetUserWidgetObject` (`self.LifeBar`))))
      (set `/Game/Blueprints/NPC/LifeBarNPC.EnemyLife` self _aslife_bar_npc))
    (:`then_1`
      (if (< (`self.Life`) 0.0)
        (`self.K2_DestroyActor`)))))

(fn `UserConstructionScript`)