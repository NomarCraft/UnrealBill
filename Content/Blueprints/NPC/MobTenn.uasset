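; MobTenn is an enemy NPC pawn that chases the player and dies when its life drops below zero.
; Tick always issues a move toward the player, turns to face them once seen, and resets movement speed, so beam slowdown is momentary.
; Capsule overlaps apply damage from two bullet types and the player's beam, gated by short delays, with a push on one bullet type.
; CheckLife handles destruction; its life bar code is disconnected.
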(event `self.PawnSensing.OnSeePawn`
  (params (Pawn :type "Pawn Object Reference"))
  (cast `/Game/Blueprints/Character/Charactertest` Pawn)
  (set `self.PlayerInSight` true))

(event `self.ReceiveTick`
  (params (DeltaSeconds :type "Float (single-precision)"))
  (bind _returnvalue (`self.K2_GetActorLocation`))
  (bind _returnvalue_2 (`AIBlueprintHelperLibrary.GetAIController` self))
  (`|ExecutionSequence`
    (:`then_0`
      (bind _ascharactertest (cast `/Game/Blueprints/Character/Charactertest` (`GameplayStatics.GetPlayerCharacter` 0)))
      ;[1 1 1] Mouvements
      (if (`self.PlayerInSight`)
        (`self.K2_SetActorRotation` (`KismetMathLibrary.FindLookAtRotation` _returnvalue (`KismetMathLibrary.MakeVector` (.x (`self.K2_GetActorLocation` _ascharactertest)) (.y (`self.K2_GetActorLocation` _ascharactertest)) (.z _returnvalue))))
        (`AITask_MoveTo.AIMoveTo` _returnvalue_2 (0.0 0.0 0.0) _ascharactertest -1.0 "Disable" "Default" true false)
        (else
          (`AITask_MoveTo.AIMoveTo` _returnvalue_2 (0.0 0.0 0.0) _ascharactertest -1.0 "Disable" "Default" true false))))
    (:`then_1`
      (`/Engine/EditorBlueprintResources/StandardMacros.DoOnce` false
        (:`Completed`
          (`self.CheckLife`))))
    (:`then_2`
      (set `FloatingPawnMovement.MaxSpeed` 200.0 (`self.FloatingPawnMovement`)))))

(event `self.Capsule.OnComponentBeginOverlap`
  (params (OverlappedComponent :type "PrimitiveComponent Object Reference") (OtherActor :type "Actor Object Reference") (OtherComp :type "PrimitiveComponent Object Reference") (OtherBodyIndex :type Integer) (bFromSweep :type Boolean) (SweepResult :type "HitResult Structure (by ref)"))
  (bind (_returnvalue_x _returnvalue_y _returnvalue_z) (`KismetMathLibrary.BreakVector` (* (`KismetMathLibrary.Normal` (- (`self.K2_GetActorLocation`) SweepResult_ImpactPoint)) 100.0)))
  ;[1 1 1] TakeDammages
  (`KismetSystemLibrary.PrintString` (`KismetSystemLibrary.GetDisplayName` OtherActor))
  (`|ExecutionSequence`
    (:`then_0`
      ;;[1 1 1] Bullet
      (if (not (`self.TimerInvisibilite`))
        (bind _asbullet_test (cast `/Game/Blueprints/Character/Bullets/BulletTest` OtherActor))
        (`/Engine/EditorBlueprintResources/StandardMacros.IsValid` _asbullet_test
          (:`Is Valid`
            (`self.K2_DestroyActor` _asbullet_test)
            (set `self.Life` (- (`self.Life`) 0.1))
            (set `self.TimerInvisibilite` true)
            (`self.K2_AddActorLocalTransform` (`KismetMathLibrary.Conv_VectorToTransform` (`KismetMathLibrary.MakeVector` _returnvalue_x _returnvalue_y _returnvalue_z)))
            (`KismetSystemLibrary.Delay` 0.2)
            (set `self.TimerInvisibilite` false)))))
    (:`then_1`
      ;;[1 1 1] Beam
      (bind _ascharactertest (cast `/Game/Blueprints/Character/Charactertest` OtherActor))
      (if (== OtherComp (`/Game/Blueprints/Character/Charactertest.BeamCylinder` _ascharactertest))
        (set `FloatingPawnMovement.MaxSpeed` 50.0 (`self.FloatingPawnMovement`))
        (if (not (`self.BEamDelay`))
          (set `self.Life` (- (`self.Life`) 0.1))
          (set `self.BEamDelay` true)
          (`KismetSystemLibrary.Delay` 0.5)
          (set `self.BEamDelay` false))))
    (:`then_2`
      ;;[1 1 1] BulletScale
      (if (not (`self.TimerInvisibilite`))
        (bind _asbullet_scale (cast `/Game/Blueprints/Character/Bullets/BulletScale` OtherActor))
        (`self.K2_DestroyActor` _asbullet_scale)
        (set `self.Life` (- (`self.Life`) 0.1))
        (set `self.TimerInvisibilite` true)
        (`KismetSystemLibrary.Delay` 0.2)
        (set `self.TimerInvisibilite` false)))
    (:`then_3`
      (`self.CheckLife`))))

(fn `CheckLife`
  (`/Engine/EditorBlueprintResources/StandardMacros.IsValid` self
    (:`Is Valid`
      (`|ExecutionSequence`
        (:`then_1`
          (if (< (`self.Life`) 0.0)
            (`self.K2_DestroyActor`)))))))

(fn `UserConstructionScript`)